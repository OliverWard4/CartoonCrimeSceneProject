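; StudyLadder is a possessable pawn for the study's movable ladder, which the player slides within a box around its start location.
; A looping timer reads LightsOn from the game instance to allow movement.
; With lights off, movement input shows a "too dark" message, or if UnderFan, a ceiling fan widget and spawned KillerNotes clue.
; That branch and Esc both animate the camera back and repossess the main character.
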(event `self.ReceiveBeginPlay`
  (set `self.startlocation` (`SceneComponent.K2_GetComponentLocation` (`self.CapsuleComponent`)))
  (`KismetSystemLibrary.K2_SetTimer` null "CanMove" 0.4 true))

(event `InputAxis|LeftRight`
  (params (AxisValue :type "Float (single-precision)"))
  (bind _returnvalue (`GameplayStatics.GetPlayerController` 0))
  (bind _original_controller (`self.Original Controller`))
  (bind _moveablearea_x (`KismetMathLibrary.BreakVector` (`self.moveableArea`)))
  (bind _mediaplayer (`self.MediaPlayer`))
  (bind _startlocation_x (`KismetMathLibrary.BreakVector` (`self.startlocation`)))
  (bind _moveablearea_x_2 (`KismetMathLibrary.BreakVector` (`self.moveableArea`)))
  (bind _startlocation_x_2 (`KismetMathLibrary.BreakVector` (`self.startlocation`)))
  (bind _returnvalue_x (`KismetMathLibrary.BreakVector` (`SceneComponent.K2_GetComponentLocation` (`self.CapsuleComponent`))))
  (bind _returnvalue_x_2 (`KismetMathLibrary.BreakVector` (`SceneComponent.K2_GetComponentLocation` (`self.CapsuleComponent`))))
  (bind _returnvalue_2 (`SceneComponent.K2_GetComponentToWorld` (`self.Ladder Camera`)))
  ;[1 1 1] Movement Bounds
  (if (`self.canMoveStairs`)
    (if (> (+ _returnvalue_x_2 1.0) (+ _startlocation_x_2 _moveablearea_x))
      (`self.AddMovementInput` (-1.0 0.0 0.0))
      (elif (< (+ _returnvalue_x -1.0) (- _startlocation_x _moveablearea_x_2))
        (`self.AddMovementInput` (1.0 0.0 0.0))
        (else
          (`self.AddMovementInput` (1.0 0.0 0.0) AxisValue))))
    (else
      ;[1 1 1] Checks If lights are on
      (if (`self.UnderFan`) :!label _label
        (if (`MediaPlayer.IsPlaying` _mediaplayer)
          (`MediaPlayer.OpenSource` _mediaplayer "/Game/Assets/Media/Animations/CeilingFanAnim.CeilingFanAnim"))
        (bind _returnvalue_3 (`|CreateWidget` "/Game/BluePrints/AnimationWidgets/CeilingFanAnim.CeilingFanAnim_C"))
        (`UserWidget.AddToViewport` _returnvalue_3 0)
        (`self.DisableInput` _returnvalue)
        (`KismetSystemLibrary.Delay` 3.0)
        (`self.EnableInput` _returnvalue)
        (bind _returnvalue_4 (`|SpawnActorFromClass` "/Game/BluePrints/KillerNotes.KillerNotes_C" (`KismetMathLibrary.MakeTransform` (-126.0 -10.0 123.0) (struct :`Yaw` -20.0)) "Undefined" "MultiplyWithRoot" null null))
        (set `/Game/BluePrints/KillerNotes.slateBrush` (`WidgetBlueprintLibrary.MakeBrushFromTexture` "/Game/Assets/Pencil.Pencil") _returnvalue_4)
        (else
          (bind _returnvalue_5 (`|CreateWidget` "/Game/BluePrints/NPC/NPC_Dialogue.NPC_Dialogue_C" (`GameplayStatics.GetPlayerController` 0)))
          (`UserWidget.AddToViewport` _returnvalue_5 0)
          (`TextBlock.SetText` (`/Game/BluePrints/NPC/NPC_Dialogue.TalkText` _returnvalue_5) "Its Too dark to Move the Stairs")
          (`KismetSystemLibrary.Delay` 2.0)
          (`WidgetLayoutLibrary.RemoveAllWidgets`)))
      (bind _asmain_charchter (cast `/Game/BluePrints/MainCharchter` _original_controller))
      (`SceneComponent.K2_SetWorldTransform` (`/Game/BluePrints/MainCharchter.Camera` _asmain_charchter) _returnvalue_2 false false)
      (set `/Game/BluePrints/MainCharchter.New Camera Location` (`/Game/BluePrints/MainCharchter.Camera Start Location` _asmain_charchter) _asmain_charchter)
      (set `/Game/BluePrints/MainCharchter.Camera Start Location` _returnvalue_2 _asmain_charchter)
      (set `/Game/BluePrints/MainCharchter.in menu` true _asmain_charchter)
      (`/Game/BluePrints/MainCharchter.Camera Move` _original_controller)
      (`Controller.Possess` (`GameplayStatics.GetPlayerController` 0) _original_controller))))

(event `InputAxis|ForwardBackward`
  (params (AxisValue :type "Float (single-precision)"))
  (bind (_startlocation_x _startlocation_y) (`KismetMathLibrary.BreakVector` (`self.startlocation`)))
  (bind (_moveablearea_x _moveablearea_y) (`KismetMathLibrary.BreakVector` (`self.moveableArea`)))
  (bind (_startlocation_x_2 _startlocation_y_2) (`KismetMathLibrary.BreakVector` (`self.startlocation`)))
  (bind (_moveablearea_x_2 _moveablearea_y_2) (`KismetMathLibrary.BreakVector` (`self.moveableArea`)))
  (bind (_returnvalue_x _returnvalue_y) (`KismetMathLibrary.BreakVector` (`SceneComponent.K2_GetComponentLocation` (`self.CapsuleComponent`))))
  (bind (_returnvalue_x_2 _returnvalue_y_2) (`KismetMathLibrary.BreakVector` (`SceneComponent.K2_GetComponentLocation` (`self.CapsuleComponent`))))
  ;[1 1 1] Movement Bounds
  (if (`self.canMoveStairs`)
    (if (> (+ _returnvalue_y 1.0) (+ _startlocation_y _moveablearea_y))
      (`self.AddMovementInput` (0.0 -1.0 0.0))
      (elif (< (+ _returnvalue_y_2 -1.0) (- _startlocation_y_2 _moveablearea_y_2))
        (`self.AddMovementInput` (0.0 1.0 0.0))
        (else
          (`self.AddMovementInput` (0.0 1.0 0.0) (* AxisValue 1.0)))))
    (else
      (goto _label))))

(event `InputAction|esc`
  (params (Key :type "Key Structure"))
  (bind _original_controller (`self.Original Controller`))
  (bind _returnvalue (`SceneComponent.K2_GetComponentToWorld` (`self.Ladder Camera`)))
  (:`Pressed`
    (bind _asmain_charchter (cast `/Game/BluePrints/MainCharchter` _original_controller))
    (`SceneComponent.K2_SetWorldTransform` (`/Game/BluePrints/MainCharchter.Camera` _asmain_charchter) _returnvalue false false)
    (set `/Game/BluePrints/MainCharchter.New Camera Location` (`/Game/BluePrints/MainCharchter.Camera Start Location` _asmain_charchter) _asmain_charchter)
    (set `/Game/BluePrints/MainCharchter.Camera Start Location` _returnvalue _asmain_charchter)
    (set `/Game/BluePrints/MainCharchter.in menu` true _asmain_charchter)
    (`/Game/BluePrints/MainCharchter.Camera Move` _original_controller)
    (`Controller.Possess` (`GameplayStatics.GetPlayerController` 0) _original_controller)))

(fn `CanMove`
  (bind _asmystery_game_instance (cast `/Game/BluePrints/MysteryGameInstance` (`GameplayStatics.GetGameInstance`)))
  (if (`/Game/BluePrints/MysteryGameInstance.LightsOn` _asmystery_game_instance)
    (set `self.canMoveStairs` true)
    (else
      (set `self.canMoveStairs` false))))

(fn `UserConstructionScript`)