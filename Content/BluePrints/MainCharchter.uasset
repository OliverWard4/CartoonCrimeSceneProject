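; Player character for a murder mystery game, handling walking, looking, a pickup flashlight, in-game menu and Y/N dialogue replies.
; Interact box-traces from the camera and branches on actor class or interface to books, notes, NPCs, bookshelf puzzle, light switch and a five-switch combination puzzle.
; Study ladder use blends the camera through a timeline before possessing the ladder.
; InMenu gates movement and look; MysteryGameInstance holds evidence and question state.
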(event `self.ReceiveBeginPlay`
  ;[1 1 1] Event Begin Play
  (bind _returnvalue (`GameplayStatics.GetCurrentLevelName` true))
  (if (`KismetStringLibrary.EqualEqual_StrStr` _returnvalue "Level1")
    (bind _returnvalue_2 (`|CreateWidget` "/Game/BluePrints/NPC/NPC_Dialogue.NPC_Dialogue_C"))
    (`UserWidget.AddToViewport` _returnvalue_2 0)
    (`TextBlock.SetText` (`/Game/BluePrints/NPC/NPC_Dialogue.TalkText` _returnvalue_2) "Where Should I start there has gotta be something around here that can lead me to the killer")
    (`KismetSystemLibrary.Delay` 3.5)
    (`TextBlock.SetText` (`/Game/BluePrints/NPC/NPC_Dialogue.TalkText` _returnvalue_2) "(Walk around with A,S,D,W and interact with 'E'  Good Luck ;) )")
    (`KismetSystemLibrary.Delay` 3.0)
    (`Widget.RemoveFromParent` _returnvalue_2)
    (`KismetSystemLibrary.K2_SetTimer` null "UpdateLightDirection" 0.001)))

(event `InputAxis|ForwardBackward`
  (params (AxisValue :type "Float (single-precision)"))
  (bind (_returnvalue_x _returnvalue_y) (`KismetMathLibrary.BreakVector` (`KismetMathLibrary.GetForwardVector` (`KismetMathLibrary.MakeRotator` 0.0 0.0 (.yaw (`self.GetControlRotation`))))))
  ;[1 1 1] move Forward/Backward
  (if (not (`self.in menu`))
    (`self.AddMovementInput` (`KismetMathLibrary.MakeVector` _returnvalue_x _returnvalue_y) (* AxisValue (`self.RunMultip`)))))

(event `InputAxis|LookUP/Down`
  (params (AxisValue :type "Float (single-precision)"))
  (bind _camera (`self.Camera`))
  (bind (_returnvalue_roll _returnvalue_pitch _returnvalue_yaw) (`KismetMathLibrary.BreakRotator` (`SceneComponent.K2_GetComponentRotation` _camera)))
  (bind _returnvalue (+ _returnvalue_pitch (`KismetMathLibrary.FClamp` AxisValue -1.0)))
  ;[1 1 1] Camera Controls
  (if (`self.in menu`)
    _
    (elif (< (`KismetMathLibrary.Abs` _returnvalue) 55.0)
      (`SceneComponent.K2_SetWorldRotation` _camera (`KismetMathLibrary.MakeRotator` _returnvalue_roll _returnvalue _returnvalue_yaw) false false))))

(event `Camera Move`
  (bind _camera_start_location (`self.Camera Start Location`))
  (bind _new_camera_location (`self.New Camera Location`))
  (bind _camera (`self.Camera`))
  (bind _camera_start_location_2 (`self.Camera Start Location`))
  (bind _new_camera_location_location (`KismetMathLibrary.BreakTransform` (`self.New Camera Location`)))
  (bind _camera_start_location_location (`KismetMathLibrary.BreakTransform` (`self.Camera Start Location`)))
  (bind _camera_start_location_location_2 (`KismetMathLibrary.BreakTransform` (`self.Camera Start Location`)))
  ;[1 1 1] Camera Smothing
  (bind (_direction _camerasmove) (`Timeline|CameraMove` :!via `PlayFromStart`)
    (:`Update`
      (`SceneComponent.K2_SetWorldLocation` _camera (+ _camera_start_location_location_2 (* _camerasmove (- _new_camera_location_location _camera_start_location_location))) false false)
      (`SceneComponent.K2_SetWorldRotation` _camera (`KismetMathLibrary.MakeRotator` (+ (* (- (.roll (.rotation _new_camera_location)) (.roll (.rotation _camera_start_location_2))) _camerasmove) (.roll (.rotation _camera_start_location))) (+ (* (- (.pitch (.rotation _new_camera_location)) (.pitch (.rotation _camera_start_location_2))) _camerasmove) (.pitch (.rotation _camera_start_location))) (+ (* (- (.yaw (.rotation _new_camera_location)) (.yaw (.rotation _camera_start_location_2))) _camerasmove) (.yaw (.rotation _camera_start_location)))) false false))
    (:`Finished`
      (set `self.in menu` false))))

(event `InputAxis|LookRight/Left`
  (params (AxisValue :type "Float (single-precision)"))
  ;[1 1 1] Camera Controls
  (if (not (`self.in menu`))
    (`self.AddControllerYawInput` (`KismetMathLibrary.FClamp` AxisValue -1.0))))

(event `InputAxis|LeftRight`
  (params (AxisValue :type "Float (single-precision)"))
  (bind (_returnvalue_x _returnvalue_y) (`KismetMathLibrary.BreakVector` (`KismetMathLibrary.GetRightVector` (`KismetMathLibrary.MakeRotator` 0.0 0.0 (.yaw (`self.GetControlRotation`))))))
  ;[1 1 1] move Forward/Backward
  (if (not (`self.in menu`))
    (`self.AddMovementInput` (`KismetMathLibrary.MakeVector` _returnvalue_x _returnvalue_y) (* AxisValue (`self.RunMultip`)))))

(event `InputAction|interact`
  (params (Key :type "Key Structure"))
  (bind _camera (`self.Camera`))
  (bind _switchtable (`self.SwitchTable`))
  (bind _switchtable_2 (`self.SwitchTable`))
  (bind _returnvalue (`SceneComponent.K2_GetComponentLocation` _camera))
  ;[1 1 1] interact
  (:`Pressed`
    (bind _outhits (`KismetSystemLibrary.BoxTraceMulti` :`Start` _returnvalue :`End` (+ (* (`KismetMathLibrary.GetForwardVector` (`SceneComponent.K2_GetComponentRotation` _camera)) 160.0) _returnvalue) :`HalfSize` (20.0 20.0 20.0) :`TraceChannel` "TraceTypeQuery1" :`DrawDebugType` "ForDuration"))
    (for _array_element _outhits
      (bind (_bblockinghit _binitialoverlap _time _distance _location _impactpoint _normal _impactnormal _physmat _hitactor) (`GameplayStatics.BreakHitResult` _array_element))
      (`KismetSystemLibrary.PrintString` (`KismetSystemLibrary.GetDisplayName` _hitactor))
      (bind _returnvalue_2 (`GameplayStatics.GetObjectClass` _hitactor))
      (if (== _returnvalue_2 "/Game/BluePrints/StudyLadder.StudyLadder_C")
        ;;[1 1 1] StudyLadder
        (bind _asstudy_ladder (cast `/Game/BluePrints/StudyLadder` _hitactor))
        (set `/Game/BluePrints/StudyLadder.Original Controller` self _asstudy_ladder)
        (set `self.Camera Start Location` (`SceneComponent.K2_GetComponentToWorld` (`self.Camera`)))
        (set `self.New Camera Location` (`SceneComponent.K2_GetComponentToWorld` (`/Game/BluePrints/StudyLadder.Ladder Camera` _asstudy_ladder)))
        (`self.Camera Move`)
        (set `self.in menu` true)
        (`KismetSystemLibrary.Delay` 2.0)
        (`Controller.Possess` (`GameplayStatics.GetPlayerController` 0) _asstudy_ladder)
        (else
          ;;[1 1 1] BookPuzzle
          (if (== _returnvalue_2 "/Game/BluePrints/BookShelf.BookShelf_C")
            (bind _returnvalue_3 (`|CreateWidget` "/Game/BluePrints/BookPuzzle.BookPuzzle_C"))
            (`UserWidget.AddToViewport` _returnvalue_3 0)
            (set `self.in menu` true)
            (set `PlayerController.bShowMouseCursor` true (`GameplayStatics.GetPlayerController` 0))
            (set `/Game/BluePrints/BookPuzzle.MainCharchterRef` self _returnvalue_3)
            (else
              ;;[1 1 1] FlashLight
              (if (`KismetSystemLibrary.DoesImplementInterface` _hitactor "/Game/BluePrints/ObjectInterface.ObjectInterface_C")
                (if (== _returnvalue_2 "/Game/BluePrints/FlashLight.FlashLight_C")
                  (bind _asflash_light (cast `/Game/BluePrints/FlashLight` _hitactor))
                  (set `self.HasFlashLight` true)
                  (`SceneComponent.SetVisibility` (`/Game/BluePrints/FlashLight.FlashLight` _asflash_light) false false)
                  (bind _returnvalue_4 (`|CreateWidget` "/Game/BluePrints/NPC/NPC_Dialogue.NPC_Dialogue_C" (`GameplayStatics.GetPlayerController` 0)))
                  (`UserWidget.AddToViewport` _returnvalue_4 0)
                  (`TextBlock.SetText` (`/Game/BluePrints/NPC/NPC_Dialogue.TalkText` _returnvalue_4) "To use the flashLight Press F")
                  (else
                    ;;[1 1 1] Light Switch
                    (if (== _returnvalue_2 "/Game/BluePrints/LightSwitch.LightSwitch_C")
                      (if (`self.HasFlashLight`)
                        (bind _asmystery_game_instance (cast `/Game/BluePrints/MysteryGameInstance` (`GameplayStatics.GetGameInstance`)))
                        (message `/Game/BluePrints/ObjectInterface.highlight` _hitactor)
                        (else
                          (bind _returnvalue_5 (`|CreateWidget` "/Game/BluePrints/NPC/NPC_Dialogue.NPC_Dialogue_C" (`GameplayStatics.GetPlayerController` 0)))
                          (`UserWidget.AddToViewport` _returnvalue_5 0)
                          (`TextBlock.SetText` (`/Game/BluePrints/NPC/NPC_Dialogue.TalkText` _returnvalue_5) "I can't see if I turn off the lights")
                          (`KismetSystemLibrary.Delay` 3.0)
                          (`WidgetLayoutLibrary.RemoveAllWidgets`)))
                      (else
                        ;;[1 1 1] Switches
                        (if (== _returnvalue_2 "/Game/BluePrints/Switches.Switches_C")
                          (bind _asswitches (cast `/Game/BluePrints/Switches` _hitactor))
                          (bind _returnvalue_6 (select `/Game/BluePrints/SwitchColor` (`/Game/BluePrints/Switches.Color` _asswitches) :`NewEnumerator1` 1 :`NewEnumerator2` 2 :`NewEnumerator3` 3 :`NewEnumerator4` 4))
                          (`KismetArrayLibrary.Array_Set` _switchtable _returnvalue_6 (not (`|GetArrayItem` _switchtable _returnvalue_6)))
                          (`SceneComponent.K2_AddWorldRotation` (`/Game/BluePrints/Switches.StaticMesh` _asswitches) (struct :`Roll` 180.0) false false)
                          (for (_ _array_index) _switchtable_2
                            (if (not (== (`|GetArrayItem` _switchtable_2 _array_index) (`|GetArrayItem` (`|MakeArray` true false false true true) _array_index)))
                              (break)))
                          (if (== _array_index 4)
                            (if (== (`|GetArrayItem` (`self.SwitchTable`) 4) true)
                              (`GameplayStatics.PlaySound2D` "/Game/Assets/Media/Sound/Bell.Bell" 1.0 1.0 4.0 null null)
                              (`SceneComponent.K2_SetWorldLocation` (`Character.CapsuleComponent` (`/Game/BluePrints/Switches.Dog` _asswitches)) (-987.05405 -528.412644 130.428728) false false)
                              (bind _returnvalue_7 (`|SpawnActorFromClass` "/Game/BluePrints/KillerNotes.KillerNotes_C" (`KismetMathLibrary.MakeTransform` (-1027.481037 -528.412644 123.625839)) "Undefined" "MultiplyWithRoot" null null))
                              (set `/Game/BluePrints/KillerNotes.slateBrush` (make `SlateBrush` "Image" "NoTile" "NoMirror" (struct :`X` 32.0 :`Y` 32.0) (struct) (struct :`SpecifiedColor` (struct :`R` 1.0 :`G` 1.0 :`B` 1.0 :`A` 1.0) :`ColorUseRule` "UseColor_Specified") (struct :`CornerRadii` (struct :`W` 1.0) :`Color` (struct :`SpecifiedColor` (struct) :`ColorUseRule` "UseColor_Specified") :`RoundingType` "HalfHeightRadius") "/Game/Assets/Pen.Pen") _returnvalue_7)))
                          (else
                            ;;[1 1 1] Book with Note
                            (if (== (`GameplayStatics.GetObjectClass` _hitactor) "/Game/BluePrints/Book.Book_C")
                              (bind _asbook (cast `/Game/BluePrints/Book` _hitactor))
                              (`/Engine/EditorBlueprintResources/StandardMacros.IsValid` (stale _returnvalue_8)
                                (:`Is Valid`
                                  (if (`Widget.IsVisible` (stale _returnvalue_8))
                                    (`Widget.SetVisibility` (stale _returnvalue_8) "Collapsed")
                                    (else
                                      (`Widget.SetVisibility` (stale _returnvalue_8) "Visible"))))
                                (:`Is Not Valid`
                                  (bind _returnvalue_8 (`|CreateWidget` "/Game/BluePrints/NPC/NPC_Dialogue.NPC_Dialogue_C" (`GameplayStatics.GetPlayerController` 0)))
                                  (`UserWidget.AddToViewport` _returnvalue_8 0)))
                              (`TextBlock.SetText` (`/Game/BluePrints/NPC/NPC_Dialogue.TalkText` _returnvalue_8) (`KismetTextLibrary.Conv_StringToText` (`/Game/BluePrints/Book.message` _asbook)))
                              (if (`KismetStringLibrary.EqualEqual_StrStr` (`/Game/BluePrints/Book.Name` _asbook) "Journal")
                                (bind _asmystery_game_instance_2 (cast `/Game/BluePrints/MysteryGameInstance` (`GameplayStatics.GetGameInstance`)))
                                (set `/Game/BluePrints/MysteryGameInstance.hasEvidence` true _asmystery_game_instance_2)
                                (`self.K2_DestroyActor` _asbook)
                                (else
                                  (`KismetSystemLibrary.Delay` 5.0)
                                  (`Widget.SetVisibility` _returnvalue_8 "Collapsed")))
                              (else
                                ;;[1 1 1] Killer Notes
                                (if (== (`GameplayStatics.GetObjectClass` _hitactor) "/Game/BluePrints/KillerNotes.KillerNotes_C")
                                  (`/Engine/EditorBlueprintResources/StandardMacros.IsValid` (stale _returnvalue_9)
                                    (:`Is Valid`
                                      (if (`Widget.IsVisible` (stale _returnvalue_9))
                                        (`Widget.SetVisibility` (stale _returnvalue_9) "Hidden")
                                        (else
                                          (`Widget.SetVisibility` (stale _returnvalue_9) "Visible")
                                          (bind _askiller_notes (cast `/Game/BluePrints/KillerNotes` _hitactor :!label _label))
                                          (`Image.SetBrush` (`/Game/BluePrints/AnimationWidgets/KillerWidget.Note` (stale _returnvalue_9)) (`/Game/BluePrints/KillerNotes.slateBrush` _askiller_notes)))))
                                    (:`Is Not Valid`
                                      (bind _returnvalue_9 (`|CreateWidget` "/Game/BluePrints/AnimationWidgets/KillerWidget.KillerWidget_C"))
                                      (`UserWidget.AddToViewport` _returnvalue_9 0)
                                      (goto _label))))))))))))
                (else
                  ;;[1 1 1] NPC
                  (if (`KismetSystemLibrary.DoesImplementInterface` _hitactor "/Game/BluePrints/NPC/Dialogue_Interface.Dialogue_Interface_C")
                    (bind _output_get (set `self.NPC` _hitactor))
                    (message `/Game/BluePrints/NPC/Dialogue_Interface.Dialogue` _output_get)))))))))))

(event `/Game/BluePrints/ObjectInterface.Return`
  ;[1 1 1] interact
  ;;[1 1 1] BookPuzzle
  (bind _asbook_shelf (cast `/Game/BluePrints/BookShelf` (`.HitActor` (`GameplayStatics.BreakHitResult` (stale `InputAction|interact` _array_element)))))
  (`StaticMeshComponent.SetStaticMesh` (`/Game/BluePrints/BookShelf.BookShelf` _asbook_shelf) "/Game/Meshes/OpenBookCase.OpenBookCase")
  (`PrimitiveComponent.SetCollisionResponseToAllChannels` (`/Game/BluePrints/BookShelf.Box` _asbook_shelf) "ECR_Overlap"))

(event `InputAction|esc`
  (params (Key :type "Key Structure"))
  ;[1 1 1] interact
  ;;[1 1 1] Quit
  (:`Pressed`
    (bind _asnpc (cast `/Game/BluePrints/NPC/NPC` (`self.NPC`)))
    (set `/Game/BluePrints/NPC/NPC.talkIndex` -1 _asnpc)
    (`Widget.SetVisibility` (`/Game/BluePrints/NPC/NPC.UI` _asnpc) "Collapsed")
    (bind _foundwidgets (`WidgetBlueprintLibrary.GetAllWidgetsOfClass` "/Game/BluePrints/NPC/NPC_Dialogue.NPC_Dialogue_C" false))
    (for _array_element _foundwidgets
      (`Widget.SetVisibility` _array_element "Collapsed"))))

(event `Key|Y`
  (params (Key :type "Key Structure"))
  (bind _npc (`self.NPC`))
  ;[1 1 1] interact
  ;;[1 1 1] Yes No Response
  (:`Pressed`
    (`/Engine/EditorBlueprintResources/StandardMacros.IsValid` "/Game/BluePrints/NPC/NPC_Dialogue.NPC_Dialogue"
      (:`Is Valid`
        (bind _asmystery_game_instance (cast `/Game/BluePrints/MysteryGameInstance` (`GameplayStatics.GetGameInstance`)))
        (if (`/Game/BluePrints/MysteryGameInstance.Interactive Question Appeared` _asmystery_game_instance)
          (message `/Game/BluePrints/NPC/Dialogue_Interface.Response` _npc "Y" self)
          (message `/Game/BluePrints/NPC/Dialogue_Interface.EndDialogue` _npc))))))

(event `Key|N`
  (params (Key :type "Key Structure"))
  ;[1 1 1] interact
  ;;[1 1 1] Yes No Response
  (:`Pressed`
    (`/Engine/EditorBlueprintResources/StandardMacros.IsValid` "/Game/BluePrints/NPC/NPC_Dialogue.NPC_Dialogue"
      (:`Is Valid`
        (bind _asmystery_game_instance (cast `/Game/BluePrints/MysteryGameInstance` (`GameplayStatics.GetGameInstance`)))
        (if (`/Game/BluePrints/MysteryGameInstance.Interactive Question Appeared` _asmystery_game_instance)
          (message `/Game/BluePrints/NPC/Dialogue_Interface.Response` (`self.NPC`) "N" self))))))

(event `InputAction|FlashLight`
  (params (Key :type "Key Structure"))
  (bind _light (`self.Light`))
  ;[1 1 1] interact
  ;;[1 1 1] Toggle Flashlight
  (:`Pressed`
    (if (`KismetSystemLibrary.IsValid` (stale `InputAction|interact` _returnvalue_4))
      (`WidgetLayoutLibrary.RemoveAllWidgets`))
    (if (`self.HasFlashLight`)
      (if (`self.LightOn`)
        (`SceneComponent.SetVisibility` _light false false)
        (set `self.LightOn` false)
        (else
          (`SceneComponent.SetVisibility` _light true false)
          (set `self.LightOn` true))))))

(event `InputAction|Menu`
  (params (Key :type "Key Structure"))
  ;[1 1 1] interact
  ;;[1 1 1] Menu
  (:`Pressed`
    (if (`KismetSystemLibrary.IsValid` (stale _returnvalue))
      (if (`Widget.IsVisible` (stale _returnvalue))
        (`Widget.SetVisibility` (stale _returnvalue) "Collapsed")
        (set `self.in menu` false)
        (else
          (`Widget.SetVisibility` (stale _returnvalue) "Visible")
          (set `self.in menu` true)))
      (else
        (bind _returnvalue (`|CreateWidget` "/Game/BluePrints/Main_Menu/InGameMenu.InGameMenu_C"))
        (`Widget.SetVisibility` _returnvalue "Visible")
        (set `/Game/BluePrints/Main_Menu/InGameMenu.Original Controller` self _returnvalue)
        (`UserWidget.AddToViewport` _returnvalue 0)
        (set `self.in menu` true)))))

(fn `UpdateLightDirection`
  (`SceneComponent.K2_SetRelativeRotation` (`self.Light`) (`SceneComponent.RelativeRotation` (`self.Camera`)) false false))

(fn `UserConstructionScript`)