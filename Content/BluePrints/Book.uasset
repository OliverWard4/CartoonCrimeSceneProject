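; Book is a selectable world prop that appears as either a killer's note or a killer's journal.
; Its Construction Script picks the BookMesh static mesh from the Name value, "Note" or "Journal".
; Selection events toggle Render Custom Depth on the mesh, the usual hook for a post-process highlight.
; IsSelected is a stub that always returns false, so the actor tracks no selection state.
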(event `/Game/BluePrints/ObjectInterface.SelectingActor`
  (`PrimitiveComponent.SetRenderCustomDepth` (`self.BookMesh`) true))

(event `/Game/BluePrints/ObjectInterface.UnSelectingActor`
  (`PrimitiveComponent.SetRenderCustomDepth` (`self.BookMesh`) false))

(fn `isSelected`
  (returns (NewParam :type Boolean))
  (return false))

(fn `UserConstructionScript`
  (if (`KismetStringLibrary.EqualEqual_StrStr` (`self.Name`) "Note")
    (`StaticMeshComponent.SetStaticMesh` (`self.BookMesh`) "/Game/Meshes/KillerNote.KillerNote")
    (elif (`KismetStringLibrary.EqualEqual_StrStr` (`self.Name`) "Journal")
      (`StaticMeshComponent.SetStaticMesh` (`self.BookMesh`) "/Game/Meshes/Killer_Journal.Killer_Journal"))))