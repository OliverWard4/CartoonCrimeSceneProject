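; NPC Blueprint for the mystery game's Grandma, Dog and Cop, selected by a character enum that also sets the flipbook.
; DialogueMethod steps through a text array in a lazily created widget.
; Grandma shows Yes/No on her exact offer line; Yes moves the camera, spawns a minigame paper character and possesses it after a delay.
; With evidence, the Cop swaps in case-closing lines and auto-advances them on delays.
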(event `/Game/BluePrints/NPC/Dialogue_Interface.Dialogue`
  (bind _ui (`self.UI`))
  (bind _returnvalue (`KismetStringLibrary.EqualEqual_StrStr` (`|GetArrayItem` (`self.Dialogue_Text`) (`self.talkIndex`)) "Wanna play a game to kill the time, I'll give you something I found if you can win. "))
  (bind _returnvalue_2 (`KismetMathLibrary.SelectFloat` 1.0 0.0 _returnvalue))
  (switch `/Game/BluePrints/NPC/CharchterList` (`self.Charchter Num`)
    (:`NewEnumerator0`
      (`self.DialogueMethod` :!label _label)
      (`Button.SetBackgroundColor` (`/Game/BluePrints/NPC/NPC_Dialogue.No` _ui) (make `LinearColor` 0.0 0.0 0.0 _returnvalue_2))
      (`Button.SetBackgroundColor` (`/Game/BluePrints/NPC/NPC_Dialogue.YesButton` _ui) (make `LinearColor` 0.0 0.0 0.0 _returnvalue_2))
      (`TextBlock.SetOpacity` (`/Game/BluePrints/NPC/NPC_Dialogue.NoText` _ui) _returnvalue_2)
      (`TextBlock.SetOpacity` (`/Game/BluePrints/NPC/NPC_Dialogue.YesText` _ui) _returnvalue_2)
      (bind _asmystery_game_instance (cast `/Game/BluePrints/MysteryGameInstance` (`GameplayStatics.GetGameInstance`)))
      (set `/Game/BluePrints/MysteryGameInstance.Interactive Question Appeared` _returnvalue _asmystery_game_instance))
    (:`NewEnumerator1`
      (`self.DialogueMethod`))
    (:`NewEnumerator2`
      (if (`/Game/BluePrints/MainCharchter.hasEvidence` (`self.Original Controller`))
        (set `self.Dialogue_Text` (`|MakeArray` "Finally We can get out of here" "Looks like that old lady went insane and killed her husband. Shes just been staring at that empty table the whole time" "Good Job"))
        (`self.DialogueMethod`)
        (`KismetSystemLibrary.Delay` 1.5)
        (`self.DialogueMethod`)
        (`KismetSystemLibrary.Delay` 4.0)
        (`self.DialogueMethod`)
        (`KismetSystemLibrary.Delay` 1.5)
        (else
          (`self.DialogueMethod`))))))

(event `/Game/BluePrints/NPC/Dialogue_Interface.EndDialogue`)

(event `/Game/BluePrints/NPC/Dialogue_Interface.Response`
  (params (NewParam :type String) (`MainChar ref` :type "/Game/BluePrints/MainCharchter Object Reference"))
  (bind _original_controller (`self.Original Controller`))
  (bind _spawn_transform (`self.Spawn Transform`))
  (bind _original_controller_2 (`self.Original Controller`))
  ;[1 1 1] Checking Character and response
  (set `self.Original Controller` `MainChar ref`)
  (switch `/Game/BluePrints/NPC/CharchterList` (`self.Charchter Num`)
    (:`NewEnumerator0`
      (switch `string` NewParam
        (:`Y`
          ;[1 1 1] Performing casts to set game states
          (`Widget.SetVisibility` (`self.UI`) "Collapsed")
          (bind _asmystery_game_instance (cast `/Game/BluePrints/MysteryGameInstance` (`GameplayStatics.GetGameInstance`)))
          (set `/Game/BluePrints/MysteryGameInstance.InMiniGame` true _asmystery_game_instance)
          (set `/Game/BluePrints/MainCharchter.in menu` true _original_controller)
          ;[1 1 1] Moving Camera to Table
          (set `/Game/BluePrints/MainCharchter.New Camera Location` (`SceneComponent.K2_GetComponentToWorld` (`self.Camera`)) _original_controller_2)
          (set `/Game/BluePrints/MainCharchter.Camera Start Location` (`SceneComponent.K2_GetComponentToWorld` (`/Game/BluePrints/MainCharchter.Camera` _original_controller)) _original_controller_2)
          (`/Game/BluePrints/MainCharchter.Camera Move` null)
          (`/Game/BluePrints/MainCharchter.Camera Move` _original_controller_2)
          (bind _returnvalue (`|SpawnActorFromClass` "/Game/MiniGame/MiniGamePaperCharchter.MiniGamePaperCharchter_C" (`KismetMathLibrary.MakeTransform` (`KismetMathLibrary.MakeVector` (.x (.location _spawn_transform)) (.y (.location _spawn_transform)) (+ (.z (.location _spawn_transform)) 1.0)) (struct :`Pitch` 90.0 :`Yaw` -90.0) (.scale _spawn_transform)) "AlwaysSpawn" "MultiplyWithRoot" null null))
          (set `/Game/MiniGame/MiniGamePaperCharchter.Original Controller` (`self.Original Controller`) _returnvalue)
          (set `/Game/MiniGame/MiniGamePaperCharchter.NPC` self _returnvalue)
          (`SceneComponent.K2_SetWorldTransform` (`/Game/MiniGame/MiniGamePaperCharchter.Paper Camera` _returnvalue) (`SceneComponent.K2_GetComponentToWorld` (`self.Camera`)) false false)
          (`KismetSystemLibrary.Delay` 2.0)
          (`Controller.Possess` (`GameplayStatics.GetPlayerController` 0) _returnvalue)
          (set `self.talkIndex` -1))
        (:`N`
          (goto _label))))))

(fn `DialogueMethod`
  (bind _ui (`self.UI`))
  (bind _result (`/Engine/EditorBlueprintResources/StandardMacros.IncrementInt` (`self.talkIndex`))
    (:`  `
      (if (< _result (`KismetArrayLibrary.Array_Length` (`self.Dialogue_Text`)))
        (`/Engine/EditorBlueprintResources/StandardMacros.IsValid` _ui
          (:`Is Valid`
            (`Widget.SetVisibility` _ui "Visible"))
          (:`Is Not Valid`
            (bind _returnvalue (`|CreateWidget` "/Game/BluePrints/NPC/NPC_Dialogue.NPC_Dialogue_C" (`GameplayStatics.GetPlayerController` 0)))
            (bind _output_get (set `self.UI` _returnvalue))
            (`UserWidget.AddToViewport` _output_get 0)))
        (`TextBlock.SetText` (`/Game/BluePrints/NPC/NPC_Dialogue.TalkText` (`self.UI`)) (`KismetTextLibrary.Conv_StringToText` (`|GetArrayItem` (`self.Dialogue_Text`) (`self.talkIndex`))))
        (else
          (`Widget.SetVisibility` _ui "Collapsed")
          (set `self.talkIndex` -1))))))

(fn `UserConstructionScript`
  (bind _flipbook (`self.FlipBook`))
  (switch `/Game/BluePrints/NPC/CharchterList` (`self.Charchter Num`)
    (:`NewEnumerator0`
      (`PaperFlipbookComponent.SetFlipbook` _flipbook "/Game/Assets/Animation/PaperFlipBooks/OldLady/OldLadyFlipbook.OldLadyFlipbook"))
    (:`NewEnumerator1`
      (`PaperFlipbookComponent.SetFlipbook` _flipbook "/Game/Assets/Animation/PaperFlipBooks/Dog/dogFlipbook.dogFlipbook"))
    (:`NewEnumerator2`
      (`PaperFlipbookComponent.SetFlipbook` _flipbook "/Game/Assets/Animation/PaperFlipBooks/Robot/robotFlipbook.robotFlipbook")
      (`SceneComponent.K2_SetRelativeLocation` _flipbook (6.224 -5.994 32.255923) false false))))