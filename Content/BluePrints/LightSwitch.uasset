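; Light switch Blueprint that toggles a referenced point light in a mystery game.
; The Highlight event flips the light's visibility based on the LightsOn flag stored in MysteryGameInstance, so the state lives on the game instance.
; Selection events toggle custom depth rendering on the switch mesh and print debug text.
; IsSelected is a stub that always returns false.
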(event `/Game/BluePrints/ObjectInterface.highlight`
  (bind _pointlightcomponent (`PointLight.PointLightComponent` (`self.LightSource`)))
  (bind _asmystery_game_instance (cast `/Game/BluePrints/MysteryGameInstance` (`GameplayStatics.GetGameInstance`)))
  (if (`/Game/BluePrints/MysteryGameInstance.LightsOn` _asmystery_game_instance)
    (`SceneComponent.SetVisibility` _pointlightcomponent false false)
    (set `/Game/BluePrints/MysteryGameInstance.LightsOn` false _asmystery_game_instance)
    (else
      (`SceneComponent.SetVisibility` _pointlightcomponent true false)
      (set `/Game/BluePrints/MysteryGameInstance.LightsOn` true _asmystery_game_instance))))

(event `/Game/BluePrints/ObjectInterface.SelectingActor`
  (`KismetSystemLibrary.PrintString` "on")
  (`PrimitiveComponent.SetRenderCustomDepth` (`self.StaticMesh`) true))

(event `/Game/BluePrints/ObjectInterface.UnSelectingActor`
  (`KismetSystemLibrary.PrintString` "off")
  (`PrimitiveComponent.SetRenderCustomDepth` (`self.StaticMesh`) false))

(fn `isSelected`
  (returns (NewParam :type Boolean))
  (return false))

(fn `UserConstructionScript`)